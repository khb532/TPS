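; Third-person shooter player Blueprint that passes weapon and health changes to the HUD.
; ChangeWeapon and MakeHpPercent cast the game mode to BP_TPSGameMode and update its MainUI, the latter after calling the parent implementation.
; Input events for fire, grenade gun and sniper are empty.
; Disconnected leftover nodes hold fire animation and weapon mesh visibility toggles that never run.
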(event Input|EnhancedActionEvents|EnhancedInputActionIA_TPSGrenadeGun
  (params (ActionValue :type Boolean) (ElapsedSeconds :type Float%20%28double-precision%29) (TriggeredSeconds :type Float%20%28double-precision%29) (InputAction :type Input%20Action%20Object%20Reference :default "/Game/TPSInput/IA_TPSGrenadeGun.IA_TPSGrenadeGun")))

(event Input|EnhancedActionEvents|EnhancedInputActionIA_TPSSniperGun
  (params (ActionValue :type Boolean) (ElapsedSeconds :type Float%20%28double-precision%29) (TriggeredSeconds :type Float%20%28double-precision%29) (InputAction :type Input%20Action%20Object%20Reference :default "/Game/TPSInput/IA_TPSSniperGun.IA_TPSSniperGun")))

(event Input|EnhancedActionEvents|EnhancedInputActionIA_TPSFire
  (params (ActionValue :type Boolean) (ElapsedSeconds :type Float%20%28double-precision%29) (TriggeredSeconds :type Float%20%28double-precision%29) (InputAction :type Input%20Action%20Object%20Reference :default "/Game/TPSInput/IA_TPSFire.IA_TPSFire")))

(event EventBeginPlay)

(event Collision|EventActorBeginOverlap
  (params (OtherActor :type Actor%20Object%20Reference)))

(event EventTick
  (params (DeltaSeconds :type Float%20%28single-precision%29)))

(event EventMakeHpPercent
  (|CallParentFunction)
  (bind _asbp_tpsgame_mode (Utilities|Casting|CastToBP_TPSGameMode (Game|GetGameMode)))
  (Default|SetHP (Variables|/Game/Blueprints/BP_TPSGameMode.BP_TPSGameMode_C|GetMainUI _asbp_tpsgame_mode) (Variables|Default|Getpercent)))

(event EventChangeWeapon
  (params (IsGrenade :type Boolean))
  (bind _asbp_tpsgame_mode (Utilities|Casting|CastToBP_TPSGameMode (Game|GetGameMode)))
  (Default|ChangeWeapon (Variables|/Game/Blueprints/BP_TPSGameMode.BP_TPSGameMode_C|GetMainUI _asbp_tpsgame_mode) IsGrenade))

(fn ConstructionScript)